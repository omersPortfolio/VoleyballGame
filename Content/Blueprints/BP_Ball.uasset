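; Thrown ball for a team beach ball game that decides scoring and the next server from what it hits, then destroys itself.
; Throw sets projectile velocity and thrower; collision hits are sorted by PlayArea or offside, sand and ocean tags.
; A play-area hit scores through BP_GameState and the thrower serves again; an out hit scores a loss and passes serve to the other team's last-listed player.
; Solo play and PracticeArea out hits just return serve to the thrower.
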(event OnComponentHit(CollisionSphere)
  (params (HitComponent :type Primitive%20Component%20Object%20Reference) (OtherActor :type Actor%20Object%20Reference) (OtherComp :type Primitive%20Component%20Object%20Reference) (NormalImpulse :type Vector :default "0, 0, 0") (Hit :type Hit%20Result%20Structure%20%28by%20ref%29))
  (bind _returnvalue (Actor|ActorHasTag OtherActor "PlayArea"))
  (bind (_oceansandoffside _isoffside) (Utilities|IsActorOffside OtherActor OtherActor OtherActor))
  (bind _returnvalue_2 (Game|GetCurrentLevelName true))
  ;[1 1 1] In a Normal Level
  (if (and (Utilities|Enum|NotEqual(Enum) _returnvalue_2 "PracticeArea") (not (Variables|Default|GetbHit)))
    ;[1 1 1] IsOffside
    (if _oceansandoffside
      ;[1 1 1] Normal Levels
      (if (CallFunction|IsTeam2Present)
        ;;[0 0 0] Handle Loss
        (Variables|Default|SetbHit true)
        (if (Variables|/Game/Blueprints/Game/BP_CharacterBase.BP_CharacterBase_C|GetbIsTeam1 (Variables|Default|GetThrower))
          (|HandleOffside :!label _label)
          (else
            (goto _label IsTeam2)))
        (else
          ;;[1 0.7865 0.7865] Team1 Player is Alone in the Game
          (Utilities|FlowControl|Delay 2.0)
          (CallFunction|SetReadytoServe (Variables|Default|GetThrower))
          (Actor|DestroyActor)))
      (else
        ;;[1 1 1] WinBranch
        (if _returnvalue
          ;;[0.4336 1 0.4546] Handle Win
          (Default|AddScoreonWin (Variables|Default|GetGameState) (CallFunction|IsTeam2Present) (Variables|/Game/Blueprints/Game/BP_CharacterBase.BP_CharacterBase_C|GetbIsTeam1 (Variables|Default|GetThrower)))
          (Variables|Default|SetbHit true)
          (Utilities|FlowControl|Delay 2.0)
          (CallFunction|ServerSetReadytoServe (Variables|Default|GetThrower))
          (Actor|DestroyActor))))
    (elif (or _isoffside _returnvalue)
      ;[1 0.6696 0.3033] Tutorial Level Behaviour
      (Utilities|FlowControl|Delay 2.0)
      (CallFunction|ServerSetReadytoServe (Variables|Default|GetThrower))
      (Actor|DestroyActor))))

(event Custom|Throw
  (params (Velocity :type Vector) (Thrower :type BP%20Character%20Base%20Object%20Reference))
  ;[1 1 1] Throw Function
  (Variables|/Script/Engine.MovementComponent|SetVelocity (Variables|Default|GetProjectileMovement) Velocity)
  (Variables|Default|SetThrower Thrower))

(event Custom|SetReadyToServe
  (params (Target :type BP%20Character%20Base%20Object%20Reference))
  ;[0 0.7442 1] Set Ready To Serve to TRUE
  (Variables|/Game/Blueprints/Game/BP_CharacterBase.BP_CharacterBase_C|SetbReadyToServe Target true))

(event Custom|Server_SetReadyToServe
  (params (Target :type BP%20Character%20Base%20Object%20Reference))
  ;[0 0.7442 1] Set Ready To Serve to TRUE
  (CallFunction|SetReadytoServe Target))

(event EventBeginPlay
  ;[1 1 1] BeginPlay
  (bind _outactors (Actor|GetAllActorsOfClass "/Game/Blueprints/Game/Team2Player.Team2Player_C"))
  (Variables|Default|SetTeam2Players _outactors)
  (bind _outactors_2 (Actor|GetAllActorsOfClass "/Game/Blueprints/Game/Team1Player.Team1Player_C"))
  (Variables|Default|SetTeam1Players _outactors_2)
  (bind _asbp_game_state (Utilities|Casting|CastToBP_GameState (Game|GetGameState)))
  (Variables|Default|SetGameState _asbp_game_state))

(fn ConstructionScript)

(fn GetRandomPlayer
  (params (PlayerType :type Array%20of%20BP%20Character%20Base%20Object%20References))
  (for _array_element PlayerType
    _)
  (return _array_element))

(fn IsTeam2Present
  (return (> (Utilities|Array|Length (Variables|Default|GetTeam2Players)) 0)))