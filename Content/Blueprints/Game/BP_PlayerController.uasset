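; Multiplayer player controller that handles team selection and character spawning.
; After a short delay it has the client show the team selection widget with a mouse cursor.
; A team pick removes the widget and calls a server event that requests a spawn from BP_MultiplayerGameMode with that team's player.
; SpawnPlayer spawns and possesses the character at the supplied transform, then has the client restore game-only input.
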(event Custom|Client_ShowMainMenu
  ;[1 1 1] Show Main Menu
  (bind _returnvalue (UserInterface|CreateWidget "/Game/Blueprints/UI/WBP_TeamSelection.WBP_TeamSelection_C"))
  (bind _output_get (Variables|Default|SetMainMenu _returnvalue))
  (UserInterface|Viewport|AddtoViewport _output_get 0)
  (Input|SetInputModeGameandUI self (Variables|Default|GetMainMenu) "DoNotLock" true)
  (Variables|Default|SetbShowMouseCursor true))

(event Custom|Client_HideMouse
  (Input|SetInputModeGameOnly self)
  (Variables|Default|SetbShowMouseCursor false))

(event Custom|Server_SpawnTeam2Player
  ;[1 1 1] Team 2 Selection and Spawning
  (Default|RequestTeam2Spawn (Variables|Default|GetGameMode) self "/Game/Blueprints/Game/Team2Player.Team2Player_C"))

(event Custom|Server_SpawnTeam1Player
  ;[1 1 1] Team 1 Selection and Spawning
  (Default|RequestTeam1Spawn (Variables|Default|GetGameMode) self "/Game/Blueprints/Game/Team1Player.Team1Player_C"))

(event EventShowMainMenu
  ;[1 1 1] Show Main Menu
  (Utilities|FlowControl|Delay 1.0)
  (CallFunction|ClientShowMainMenu))

(event EventBeginPlay
  ;[1 1 1] BeginPlay
  (bind _asbp_multiplayer_game_mode (Utilities|Casting|CastToBP_MultiplayerGameMode (Game|GetGameMode)))
  (Variables|Default|SetGameMode _asbp_multiplayer_game_mode)
  (bind _asbp_game_state (Utilities|Casting|CastToBP_GameState (Game|GetGameState)))
  (bind _output_get (Variables|Default|SetGameState _asbp_game_state))
  (Development|PrintString (Utilities|GetDisplayName _output_get)))

(event EventSpawnPlayer
  (params (Player :type BP%20Character%20Base%20Class%20Reference) (Transform :type Transform))
  ;[1 1 1] Spawn Player
  (bind _returnvalue (Game|SpawnActorfromClass Player Transform "AdjustIfPossibleButAlwaysSpawn" 0 0))
  (bind _output_get (Variables|Default|SetPlayerCharacter _returnvalue))
  (Pawn|Possess _output_get)
  (CallFunction|ClientHideMouse))

(event EventTeam1Selected
  ;[1 1 1] Team 1 Selection and Spawning
  (Widget|RemovefromParent (Variables|Default|GetMainMenu))
  (CallFunction|ServerSpawnTeam1Player))

(event EventTeam2Selected
  ;[1 1 1] Team 2 Selection and Spawning
  (Widget|RemovefromParent (Variables|Default|GetMainMenu))
  (CallFunction|ServerSpawnTeam2Player))

(fn ConstructionScript)