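; Base player character for a networked ball game, with serve, throw, pass and dunk actions plus level-dependent HUD and a VSync toggle.
; An overlap volume tracks the nearby ball and gates throw, pass and dunk, while serving spawns a new ball.
; Server events launch the ball and multicast a sound.
; Holding serve re-runs projectile prediction each frame through a Delay loop, placing a landing decal until release or cancel.
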(event OnComponentEndOverlap(Collision)
  (params (OverlappedComponent :type Primitive%20Component%20Object%20Reference) (OtherActor :type Actor%20Object%20Reference) (OtherComp :type Primitive%20Component%20Object%20Reference) (OtherBodyIndex :type Integer))
  ;[1 1 1] EndOverlap
  (if (== OtherActor (Variables|Default|GetBall))
    (Variables|Booleans|SetbCanThrow false)))

(event OnComponentBeginOverlap(Collision)
  (params (OverlappedComponent :type Primitive%20Component%20Object%20Reference) (OtherActor :type Actor%20Object%20Reference) (OtherComp :type Primitive%20Component%20Object%20Reference) (OtherBodyIndex :type Integer) (bFromSweep :type Boolean) (SweepResult :type Hit%20Result%20Structure%20%28by%20ref%29))
  ;[1 1 1] BeginOverlap for CanThrow
  (if (Actor|ActorHasTag OtherActor "Ball")
    (bind _asbp_ball (Utilities|Casting|CastToBP_Ball OtherActor))
    (Variables|Default|SetBall _asbp_ball)
    (Variables|Booleans|SetbCanThrow true)))

(event Custom|Multicast_PlaySound
  ;[1 1 1] Play Sound_Multicast
  (Audio|PlaySoundatLocation "/Game/Audio/Cue_He.Cue_He" (Transformation|GetActorLocation) "0, 0, 0" 1.0 1.0 0.0 0 0 0))

(event EventBeginPlay
  (bind _returnvalue (Game|GetCurrentLevelName true))
  (if (Utilities|Enum|NotEqual(Enum) _returnvalue "PracticeArea")
    (bind _returnvalue_2 (UserInterface|CreateWidget "/Game/Blueprints/UI/WBP_UI.WBP_UI_C"))
    (UserInterface|Viewport|AddtoViewport _returnvalue_2 0)
    (else
      (bind _returnvalue_3 (UserInterface|CreateWidget "/Game/Blueprints/UI/WBP_Crosshair.WBP_Crosshair_C"))
      (UserInterface|Viewport|AddtoViewport _returnvalue_3 0))))

(event Input|ActionEvents|InputActionToggleVSync
  (params (Key :type Key%20Structure :default "None"))
  (:Pressed
    (if (Variables|Booleans|GetbVsyncOn)
      (Development|ExecuteConsoleCommand "r.VSync 1" 0)
      (else
        (Development|ExecuteConsoleCommand "r.VSync 0" 0)))))

(fn ConstructionScript)

(event Custom|Server_Dunk
  (params (Velocity :type Vector))
  ;[1 1 1] Server Dunk
  (if (Variables|Booleans|GetbCanThrow)
    (Default|Throw (Variables|Default|GetBall) Velocity self)
    (Networking|SwitchHasAuthority
      (:Authority
        (CallFunction|MulticastPlaySound)))))

(event Input|ActionEvents|InputActionDunk
  (params (Key :type Key%20Structure :default "None"))
  ;[1 1 1] Dunk
  (:Pressed
    (if (and (not (Variables|Booleans|GetbDunking)) (Variables|Booleans|GetbCanThrow))
      (Variables|Vectors|SetDunkVelocity (* (Math|Vector|GetForwardVector (Pawn|GetControlRotation :!class /Script/Engine.Pawn)) (Variables|Floats|GetDunkStrength)))
      (Variables|Booleans|SetbDunking true)
      (if (Variables|Booleans|GetbDunking)
        (CallFunction|ServerDunk (Variables|Vectors|GetDunkVelocity)))))
  (:Released
    (Variables|Booleans|SetbDunking false)))

(event Custom|Server_ThrowBall
  (params (Velocity :type Vector))
  ;[1 1 1] Server_ThrowBall
  (if (Variables|Booleans|GetbCanThrow)
    (Default|Throw (Variables|Default|GetBall) Velocity self)
    (Networking|SwitchHasAuthority
      (:Authority
        (CallFunction|MulticastPlaySound)))))

(event Input|ActionEvents|InputActionThrow
  (params (Key :type Key%20Structure :default "None"))
  (:Pressed
    (Variables|Booleans|SetbThrowing true)
    (if (and (Variables|Booleans|GetbThrowing) (Variables|Booleans|GetbCanThrow))
      (|PredictBallPath_2)))
  (:Released
    (if (Variables|Booleans|GetbCanThrow)
      (Variables|Booleans|SetbThrowing false)
      (Rendering|SetVisibility (Variables|Default|GetHitDecal) false false)
      (CallFunction|ServerThrowBall (Variables|Vectors|GetServeVelocity)))))

(event Custom|Server_Pass
  (params (Velocity :type Vector))
  (if (Variables|Booleans|GetbCanThrow)
    (Default|Throw (Variables|Default|GetBall) Velocity self)
    (Networking|SwitchHasAuthority
      (:Authority
        (CallFunction|MulticastPlaySound)))))

(event Input|ActionEvents|InputActionPass
  (params (Key :type Key%20Structure :default "None"))
  (:Pressed
    (if (and (Variables|Booleans|GetbCanThrow) (not (Variables|Booleans|GetbPassing)))
      (Variables|Vectors|SetPassVelocity (* "0, 0,1.000000" (Variables|Floats|GetPassStrength)))
      (Variables|Booleans|SetbPassing true)
      (if (Variables|Booleans|GetbPassing)
        (CallFunction|ServerPass (Variables|Vectors|GetPassVelocity)))))
  (:Released
    (Variables|Booleans|SetbPassing false)))

(event Custom|Server_ServeBall
  (params (StartPoint :type Vector) (Launch%20Velocity :type Vector))
  ;[1 1 1] Server_ServeBall
  (bind _returnvalue (Game|SpawnActorfromClass "/Game/Blueprints/BP_Ball.BP_Ball_C" (Math|Transform|MakeTransform StartPoint "0, 0, 0" "1,1,1") "AlwaysSpawn" 0 0))
  (Default|Throw _returnvalue Launch%20Velocity self)
  (Networking|SwitchHasAuthority
    (:Authority
      (CallFunction|MulticastPlaySound))))

(event Input|ActionEvents|InputActionCancel
  (params (Key :type Key%20Structure :default "None"))
  ;[1 1 1] Cancel Serving
  (:Pressed
    (if (Variables|Booleans|GetbServing)
      (Variables|Booleans|SetbCanceled true)
      (Variables|Booleans|SetbServing false)
      (Rendering|SetVisibility (Variables|Default|GetHitDecal) false false))))

(event Input|ActionEvents|InputActionServe
  (params (Key :type Key%20Structure :default "None"))
  (:Pressed
    (if (Pawn|IsLocallyControlled)
      (if (Variables|Booleans|GetbReadyToServe)
        (Variables|Booleans|SetbServing true)
        (Variables|Booleans|SetbCanceled false)
        (if (Variables|Booleans|GetbServing) :!label _label
          (bind (_outhit _outpathpositions _outlasttracedestination) (|PredictBallPath))
          (|HitPoint _outlasttracedestination)
          (for _array_element _outpathpositions
            _)
          (Utilities|FlowControl|Delay (Utilities|Time|GetWorldDeltaSeconds))
          (goto _label))
        (else
          (Development|PrintString "Not ready to serve")))))
  (:Released
    (if (Variables|Booleans|GetbServing)
      (if (not (Variables|Booleans|GetbCanceled))
        (Variables|Booleans|SetbServing false)
        (Rendering|SetVisibility (Variables|Default|GetHitDecal) false false)
        (CallFunction|ServerServeBall (Transformation|GetWorldLocation (Variables|Default|GetServeLocation)) (Variables|Vectors|GetServeVelocity))
        (Variables|Booleans|SetbReadyToServe false)))))