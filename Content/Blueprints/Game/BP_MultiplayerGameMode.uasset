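; Multiplayer game mode that handles player login and team-based spawning for two teams.
; On login it tells each new player to show the main menu, and on BeginPlay it caches all Team 1 and Team 2 start actors.
; Spawn request events pick a random start for the requested team and pass its transform to the player controller's spawn message.
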(event Custom|RequestTeam2Spawn
  (params (PlayerController :type BP%20Player%20Controller%20Object%20Reference) (Player :type Team%202%20Player%20Class%20Reference))
  (bind _team2starts (Variables|Default|GetTeam2Starts))
  (Class|INTPlayerController|SpawnPlayer(Message) PlayerController Player (Transformation|GetActorTransform (Utilities|Array|Get(acopy) _team2starts (Math|Random|RandomIntegerinRange 0 (- (Utilities|Array|Length _team2starts) 1))))))

(event Custom|RequestTeam1Spawn
  (params (PlayerController :type BP%20Player%20Controller%20Object%20Reference) (Player :type Team%201%20Player%20Class%20Reference))
  (bind _team1starts (Variables|Default|GetTeam1Starts))
  (Class|INTPlayerController|SpawnPlayer(Message) PlayerController Player (Transformation|GetActorTransform (Utilities|Array|Get(acopy) _team1starts (Math|Random|RandomIntegerinRange 0 (- (Utilities|Array|Length _team1starts) 1))))))

(event EventBeginPlay
  (Utilities|FlowControl|Sequence
    (:then_0
      (bind _outactors (Actor|GetAllActorsOfClass "/Game/Blueprints/BP_Team1Start.BP_Team1Start_C"))
      (Variables|Default|SetTeam1Starts _outactors))
    (:then_1
      (bind _outactors_2 (Actor|GetAllActorsOfClass "/Game/Blueprints/BP_Team2Start.BP_Team2Start_C"))
      (Variables|Default|SetTeam2Starts _outactors_2))))

(event EventPostLogin
  (params (NewPlayer :type Player%20Controller%20Object%20Reference))
  (Class|INTPlayerController|ShowMainMenu(Message) NewPlayer))

(fn ConstructionScript)