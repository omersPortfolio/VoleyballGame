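; Multiplayer GameInstance that manages session hosting, joining, searching and leaving through Advanced Sessions nodes.
; Hosting creates a session, stores the server settings and opens their map, while joining hides the cursor and switches to game-only input.
; Searches broadcast results through ServerFound on success or failure.
; Quitting destroys the session and opens the multiplayer main menu either way, and network errors print the failure before taking that same path.
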(event Custom|HostServer
  (params (PlayerController :type Player%20Controller%20Object%20Reference) (ServerSettings :type Server%20Settings%20Structure))
  (bind (_mapname _publicconnections _serversettings) (Utilities|Struct|BreakServerSettings ServerSettings))
  ;[1 1 1] Host Server
  (bind _output_get (Variables|Default|SetOwnerRef PlayerController))
  (|AdvancedSession _serversettings _output_get 5 0 false true false true true false false false true
    (:OnSuccess
      (Variables|Default|SetServerSettings ServerSettings)
      (Game|OpenLevel(byName) _mapname true "listen"))
    (:OnFailure
      (Development|PrintString "Failed to create session"))))

(event Custom|JoinServer
  (params (PlayerController :type Player%20Controller%20Object%20Reference) (SearchResult :type Blueprint%20Session%20Result%20Structure%20%28by%20ref%29))
  ;[1 1 1] Join Server
  (bind _output_get (Variables|Default|SetOwnerRef PlayerController))
  (|JoinSession _output_get SearchResult
    (:OnSuccess
      (Variables|/Script/Engine.PlayerController|SetbShowMouseCursor (Variables|Default|GetOwnerRef) false)
      (Input|SetInputModeGameOnly (Variables|Default|GetOwnerRef)))))

(event Custom|FindServers
  (params (PlayerController :type Player%20Controller%20Object%20Reference) (MaxResults :type Integer))
  ;[1 1 1] Find Servers
  (bind _results (|FindSessionsAdvanced PlayerController MaxResults false "AllServers" 0 false false false)
    (:OnSuccess
      _)
    (:OnFailure
      _))
  (Default|CallServerFound _results))

(event Custom|QuitToMenu
  (params (PlayerController :type Player%20Controller%20Object%20Reference))
  ;[1 1 1] Quit To Menu
  (|DestroySession PlayerController
    (:OnSuccess
      _)
    (:OnFailure
      _))
  (Game|OpenLevel(byName) "MultiplayerMainMenu"))

(event EventHandleNetworkError
  (params (FailureType :type ENetworkFailure%20Enum :default "NetDriverAlreadyExists") (bIsServer :type Boolean))
  (bind _ownerref (Variables|Default|GetOwnerRef))
  ;[1 1 1] Handle Network Error
  (Development|PrintString (Utilities|String|Append (Utilities|String|EnumtoString FailureType) " 
" (Utilities|GetDisplayName _ownerref)))
  (CallFunction|QuittoMenu _ownerref))