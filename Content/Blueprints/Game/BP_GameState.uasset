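; Game state Blueprint that keeps the scores for two teams in a game played around a thrower.
; A win event adds a point to the thrower's team, while a loss event adds one to the opposing team.
; Both events change scores only with authority and only when Team 2 is present.
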(event Custom|AddScoreOnWin
  (params (IsTeam2Present :type Boolean) (IsThrowerTeam1 :type Boolean))
  ;[1 1 1] Add Score On Win
  (Networking|SwitchHasAuthority
    (:Authority
      (if IsTeam2Present
        (if IsThrowerTeam1
          (Math|Integer|IncrementInt (Variables|Default|GetTeam1Score))
          (else
            (Math|Integer|IncrementInt (Variables|Default|GetTeam2Score))))))))

(event Custom|AddScoreOnLoss
  (params (IsTeam2Present :type Boolean) (IsThrowerTeam1 :type Boolean))
  ;[1 1 1] Add Score on Loss
  (Networking|SwitchHasAuthority
    (:Authority
      (if IsTeam2Present
        (if IsThrowerTeam1
          (Math|Integer|IncrementInt (Variables|Default|GetTeam2Score))
          (else
            (Math|Integer|IncrementInt (Variables|Default|GetTeam1Score))))))))

(fn ConstructionScript)